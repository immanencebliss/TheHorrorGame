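; Portal math function library that maps locations, directions, rotations and velocities from one portal's space into a target portal's space.
; Conversions go into the current portal's local space, flip X and Y for a half turn, then out through the target; a mirrored location variant flips only Y.
; Rotation and velocity reuse the direction conversion, with velocity keeping its speed.
; Two visibility checks test player camera distance and whether the camera is in front of an actor.
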(fn PortalConvertDirection
  (params (CurrentPortal :type BP%20Portal%20Object%20Reference) (TargetPortal :type BP%20Portal%20Object%20Reference) (PrevDirection :type Vector))
  (bind _output_get (LocalVariables|SetDirection (Math|Transform|TransformDirection (Transformation|GetActorTransform TargetPortal) (Math|Vector|MirrorVectorbyNormal (Math|Vector|MirrorVectorbyNormal (Math|Transform|InverseTransformDirection (Transformation|GetActorTransform CurrentPortal) PrevDirection) "1.000000, 0, 0") "0.000000,1.000000, 0"))))
  (return _output_get))

(fn PortalConvertLocation
  (params (CurrentPortal :type BP%20Portal%20Object%20Reference) (TargetPortal :type BP%20Portal%20Object%20Reference) (PrevLocation :type Vector))
  (bind _returnvalue (Transformation|GetActorTransform CurrentPortal))
  (bind (_location _rotation _scale) (Math|Transform|BreakTransform _returnvalue))
  (bind _output_get (LocalVariables|SetLocation (Math|Transform|TransformLocation (Transformation|GetActorTransform TargetPortal) (Math|Transform|InverseTransformLocation (Math|Transform|MakeTransform _location _rotation (Math|Vector|MakeVector (* (.x _scale) -1.0) (* (.y _scale) -1.0) (.z _scale))) PrevLocation))))
  (return _output_get))

(fn PortalConvertLocationMirrored
  (params (CurrentPortal :type BP%20Portal%20Object%20Reference) (TargetPortal :type BP%20Portal%20Object%20Reference) (PrevLocation :type Vector))
  (bind _returnvalue (Transformation|GetActorTransform CurrentPortal))
  (bind (_location _rotation _scale) (Math|Transform|BreakTransform _returnvalue))
  (bind _output_get (LocalVariables|SetLocation (Math|Transform|TransformLocation (Transformation|GetActorTransform TargetPortal) (Math|Transform|InverseTransformLocation (Math|Transform|MakeTransform _location _rotation (Math|Vector|MakeVector (.x _scale) (* (.y _scale) -1.0) (.z _scale))) PrevLocation))))
  (return _output_get))

(fn PortalConvertRotation
  (params (CurrentPortal :type BP%20Portal%20Object%20Reference) (TargetPortal :type BP%20Portal%20Object%20Reference) (PrevRotation :type Rotator))
  (bind (_x _y) (Math|Rotator|GetAxes PrevRotation))
  (bind _newdirection (Portals|PortalConvertDirection CurrentPortal TargetPortal _x))
  (LocalVariables|SetDirX _newdirection)
  (bind _newdirection_2 (Portals|PortalConvertDirection CurrentPortal TargetPortal _y))
  (LocalVariables|SetDirY _newdirection_2)
  (bind _output_get (LocalVariables|SetRotation (Math|Rotator|MakeRotfromXY (LocalVariables|GetDirX) (LocalVariables|GetDirY))))
  (return _output_get))

(fn PortalConvertVelocity
  (params (CurrentPortal :type BP%20Portal%20Object%20Reference) (TargetPortal :type BP%20Portal%20Object%20Reference) (PrevVelocity :type Vector))
  (LocalVariables|SetVelocitySize (Math|Vector|VectorLength PrevVelocity))
  (bind _newdirection (Portals|PortalConvertDirection CurrentPortal TargetPortal (Math|Vector|Normalize PrevVelocity)))
  (LocalVariables|SetVelocityDirection _newdirection)
  (bind _output_get (LocalVariables|SetVelocity (* (LocalVariables|GetVelocityDirection) (LocalVariables|GetVelocitySize))))
  (return _output_get))

(fn CheckVisibilitybyDistance
  (params (MaxRenderDistance :type Float%20%28single-precision%29) (ActorLocation :type Vector))
  (if (<= (Math|Vector|VectorLength (- (Camera|GetCameraLocation (Game|GetPlayerCameraManager 0)) ActorLocation)) MaxRenderDistance)
    (LocalVariables|SetbIsVisible true)
    (else
      (LocalVariables|SetbIsVisible false)))
  (return (LocalVariables|GetbIsVisible)))

(fn CheckVisibilitybyDirection
  (params (ActorLocation :type Vector) (ActorForwardVector :type Vector))
  (if (>= (Math|Vector|DotProduct (- (Camera|GetCameraLocation (Game|GetPlayerCameraManager 0)) ActorLocation) ActorForwardVector) 0.0)
    (LocalVariables|SetbIsVisible true)
    (else
      (LocalVariables|SetbIsVisible false)))
  (return (LocalVariables|GetbIsVisible)))