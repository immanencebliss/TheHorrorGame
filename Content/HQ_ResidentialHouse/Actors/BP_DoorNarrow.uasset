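; BP_DoorNarrow is a narrow door actor that opens or closes when the player interacts with it.
; BeginPlay caches the skeletal mesh's AnimBPDoorNarrow instance, and Interact toggles its PlayerNear flag to drive the animation.
; SlamDoor saves the current play rate, sets a tiny positive or negative rate, and forces PlayerNear according to SlamClosed.
; The saved rate is never restored here.
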(event Custom|Slam%20Door
  (params (SlamClosed? :type Boolean))
  ;[1 1 1] SLAM DOOR
  (Variables|Default|SetNormalRate (Components|Animation|GetPlayRate (Variables|Default|GetDoor_narrow)))
  (bind _output_get (Variables|Default|SetDoorOpen SlamClosed?))
  (if _output_get
    (Components|Timeline|SetPlayRate (Variables|Default|GetDoor_narrow) 0.01)
    (Variables|/Game/HQ_ResidentialHouse/Meshes/DoorNarrow/AnimBPDoorNarrow.AnimBPDoorNarrow_C|SetPlayerNear (Variables|Default|GetCastToDoorAnimation) false)
    (else
      (Components|Timeline|SetPlayRate (Variables|Default|GetDoor_narrow) -0.01)
      (Variables|/Game/HQ_ResidentialHouse/Meshes/DoorNarrow/AnimBPDoorNarrow.AnimBPDoorNarrow_C|SetPlayerNear (Variables|Default|GetCastToDoorAnimation) true))))

(event EventBeginPlay
  (bind _asanim_bpdoor_narrow (Utilities|Casting|CastToAnimBPDoorNarrow (Components|SkeletalMesh|GetAnimInstance (Variables|Default|GetDoor_narrow))))
  (Variables|Default|SetCastToDoorAnimation _asanim_bpdoor_narrow))

(event Collision|EventActorBeginOverlap
  (params (OtherActor :type Actor%20Object%20Reference)))

(event EventTick
  (params (DeltaSeconds :type Float%20%28single-precision%29)))

(event EventInteract
  (params (HitComponent :type Actor%20Component%20Object%20Reference))
  ;[1 1 1] Open and closes door when player interacts with it
  (if (Variables|/Game/HQ_ResidentialHouse/Meshes/DoorNarrow/AnimBPDoorNarrow.AnimBPDoorNarrow_C|GetPlayerNear (Variables|Default|GetCastToDoorAnimation))
    ;;[1 1 1] Close Door
    (Variables|/Game/HQ_ResidentialHouse/Meshes/DoorNarrow/AnimBPDoorNarrow.AnimBPDoorNarrow_C|SetPlayerNear (Variables|Default|GetCastToDoorAnimation) false)
    (else
      ;;[1 1 1] Open Door
      (Variables|/Game/HQ_ResidentialHouse/Meshes/DoorNarrow/AnimBPDoorNarrow.AnimBPDoorNarrow_C|SetPlayerNear (Variables|Default|GetCastToDoorAnimation) true))))

(fn ConstructionScript)