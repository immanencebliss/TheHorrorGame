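; Desk lamp actor for a residential house that toggles on and off through Interact and supports long, short and looping flicker effects.
; Construction script caches its spotlights and default intensity, creates a dynamic bulb material and applies the initial IsOff state.
; Flicker events play timelines forward or reversed to lerp light intensity and bulb emission together.
; IFlickerOff stops the looping flicker and sets the lights fully on or off.
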(event EventInteract
  (params (HitComponent :type Actor%20Component%20Object%20Reference))
  (bind _spotlight (Variables|Default|GetSpotLight))
  (if (Variables|Default|GetisOff?)
    (Rendering|Components|Light|SetIntensity _spotlight (Variables|Default|GetDefault%20intensity))
    (Rendering|Material|SetScalarParameterValue (Variables|Default|Getmat%20instance) "Emission Intensity" 15.0 :!class /Script/Engine.MaterialInstanceDynamic)
    (Variables|Default|SetIsOff? false)
    (else
      (Rendering|Components|Light|SetIntensity _spotlight 0.0)
      (Rendering|Material|SetScalarParameterValue (Variables|Default|Getmat%20instance) "Emission Intensity" 0.0 :!class /Script/Engine.MaterialInstanceDynamic)
      (Variables|Default|SetIsOff? true))))

(event EventIFlickerLong
  (params (FlickOn :type Boolean))
  (bind _output_get (Variables|Default|SetFlickOn FlickOn))
  (if _output_get
    (bind _brightness (Timeline|Timeline_3 ReverseFromEnd)
      (:Update
        (for _array_element (Variables|Default|Getspotlights)
          (Rendering|Components|Light|SetIntensity _array_element (Math|Float|Lerp 0.0 (Variables|Default|GetDefault%20Intensity) (/ _brightness 1e+01)))
          (if (Variables|Default|GetFlickOn)
            (Rendering|Material|SetScalarParameterValue (Variables|Default|Getmat%20instance) "Emission Intensity" (Math|Float|Lerp 0.0 15.0 (/ _brightness 1e+01)) :!class /Script/Engine.MaterialInstanceDynamic)
            (Variables|Default|SetIsOff? false)
            (else
              (Rendering|Material|SetScalarParameterValue (Variables|Default|Getmat%20instance) "Emission Intensity" (Math|Float|Lerp 0.0 15.0 (/ _brightness 1e+01)) :!class /Script/Engine.MaterialInstanceDynamic)
              (Variables|Default|SetIsOff? true))))))
    (else
      (Timeline|Timeline_3 PlayFromStart))))

(event EventIFlickerShort
  (params (FlickOn :type Boolean))
  ;[1 1 1] Flicker lights Short
  (bind _output_get (Variables|Default|SetFlickOn FlickOn))
  (if _output_get
    (bind _flicker_style_1 (Timeline|Timeline_4 ReverseFromEnd)
      (:Update
        (for _array_element (Variables|Default|Getspotlights)
          (Rendering|Components|Light|SetIntensity _array_element (Math|Float|Lerp 0.0 (Variables|Default|GetDefault%20Intensity) _flicker_style_1))
          (if (Variables|Default|GetFlickOn)
            (Rendering|Material|SetScalarParameterValue (Variables|Default|Getmat%20instance) "Emission Intensity" (Math|Float|Lerp 0.0 15.0 _flicker_style_1) :!class /Script/Engine.MaterialInstanceDynamic)
            (Variables|Default|SetIsOff? false)
            (else
              (Rendering|Material|SetScalarParameterValue (Variables|Default|Getmat%20instance) "Emission Intensity" (Math|Float|Lerp 0.0 15.0 _flicker_style_1) :!class /Script/Engine.MaterialInstanceDynamic)
              (Variables|Default|SetIsOff? true))))))
    (else
      (Timeline|Timeline_4 PlayFromStart))))

(event EventIFlickeron
  (params (FlickOn :type Boolean))
  ;[1 1 1] Flicker lights Looping
  (bind _output_get (Variables|Default|SetFlickOn FlickOn))
  (if _output_get
    (bind _newtrack_0 (Timeline|Timeline_2 ReverseFromEnd)
      (:Update
        (for _array_element (Variables|Default|Getspotlights)
          (Rendering|Components|Light|SetIntensity _array_element (Math|Float|Lerp 0.0 (Variables|Default|GetDefault%20Intensity) _newtrack_0))
          (if (Variables|Default|GetFlickOn)
            (Rendering|Material|SetScalarParameterValue (Variables|Default|Getmat%20instance) "Emission Intensity" (Math|Float|Lerp 0.0 15.0 _newtrack_0) :!class /Script/Engine.MaterialInstanceDynamic)
            (Variables|Default|SetIsOff? false)
            (else
              (Rendering|Material|SetScalarParameterValue (Variables|Default|Getmat%20instance) "Emission Intensity" (Math|Float|Lerp 0.0 15.0 _newtrack_0) :!class /Script/Engine.MaterialInstanceDynamic)
              (Variables|Default|SetIsOff? true))))))
    (else
      (Timeline|Timeline_2 PlayFromStart))))

(event EventIFlickerOff
  (params (FlickOn :type Boolean))
  ;[1 1 1] Flicker lights Looping
  (Utilities|FlowControl|Sequence
    (:then_0
      (bind _newtrack_0 (Timeline|Timeline_2 Stop)
        (:Update
          (for _array_element (Variables|Default|Getspotlights)
            (Rendering|Components|Light|SetIntensity _array_element (Math|Float|Lerp 0.0 (Variables|Default|GetDefault%20Intensity) _newtrack_0))
            (if (Variables|Default|GetFlickOn)
              (Rendering|Material|SetScalarParameterValue (Variables|Default|Getmat%20instance) "Emission Intensity" (Math|Float|Lerp 0.0 15.0 _newtrack_0) :!class /Script/Engine.MaterialInstanceDynamic)
              (Variables|Default|SetIsOff? false)
              (else
                (Rendering|Material|SetScalarParameterValue (Variables|Default|Getmat%20instance) "Emission Intensity" (Math|Float|Lerp 0.0 15.0 _newtrack_0) :!class /Script/Engine.MaterialInstanceDynamic)
                (Variables|Default|SetIsOff? true)))))))
    (:then_1
      (if FlickOn
        (for _array_element_2 (Variables|Default|Getspotlights)
          (Rendering|Components|Light|SetIntensity _array_element_2 (Variables|Default|GetDefault%20Intensity))
          (if (Variables|Default|GetFlickOn)
            (Rendering|Material|SetScalarParameterValue (Variables|Default|Getmat%20instance) "Emission Intensity" (Math|Float|Lerp 0.0 15.0 _newtrack_0) :!class /Script/Engine.MaterialInstanceDynamic)
            (Variables|Default|SetIsOff? false)
            (else
              (Rendering|Material|SetScalarParameterValue (Variables|Default|Getmat%20instance) "Emission Intensity" (Math|Float|Lerp 0.0 15.0 _newtrack_0) :!class /Script/Engine.MaterialInstanceDynamic)
              (Variables|Default|SetIsOff? true))))
        (else
          (for _array_element_3 (Variables|Default|Getspotlights)
            (Rendering|Components|Light|SetIntensity _array_element_3 0.0)
            (if (Variables|Default|GetFlickOn)
              (Rendering|Material|SetScalarParameterValue (Variables|Default|Getmat%20instance) "Emission Intensity" (Math|Float|Lerp 0.0 15.0 _newtrack_0) :!class /Script/Engine.MaterialInstanceDynamic)
              (Variables|Default|SetIsOff? false)
              (else
                (Rendering|Material|SetScalarParameterValue (Variables|Default|Getmat%20instance) "Emission Intensity" (Math|Float|Lerp 0.0 15.0 _newtrack_0) :!class /Script/Engine.MaterialInstanceDynamic)
                (Variables|Default|SetIsOff? true)))))))))

(fn ConstructionScript
  (bind _lampdesk_bulb (Variables|Default|GetLampDesk_Bulb))
  (Utilities|FlowControl|Sequence
    (:then_0
      (bind _output_get (Variables|Default|Setspotlights (Actor|GetComponentsByClass "/Script/Engine.SpotLightComponent")))
      (Variables|Default|SetDefault%20intensity (Variables|/Script/Engine.LightComponentBase|GetIntensity (Utilities|Array|Get(acopy) _output_get))))
    (:then_1
      (bind _returnvalue (Rendering|Material|CreateDynamicMaterialInstance _lampdesk_bulb 0 (Rendering|Material|GetMaterial _lampdesk_bulb 0) "None" :!class /Script/Engine.PrimitiveComponent))
      (Variables|Default|Setmat%20instance _returnvalue)
      (for _array_element (Variables|Default|Getspotlights)
        (if (Variables|Default|GetIsOff?)
          (Rendering|Components|Light|SetIntensity _array_element 0.0)
          (Rendering|Material|SetScalarParameterValue (Variables|Default|Getmat%20instance) "Emission Intensity" 0.0 :!class /Script/Engine.MaterialInstanceDynamic)
          (else
            (Rendering|Components|Light|SetIntensity _array_element (Variables|Default|GetDefault%20intensity))
            (Rendering|Material|SetScalarParameterValue (Variables|Default|Getmat%20instance) "Emission Intensity" 15.0 :!class /Script/Engine.MaterialInstanceDynamic)))))))