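; BP_DoorMain is a residential house main door actor, built to swing open and closed through an animation Blueprint on its DoorMain mesh.
; On BeginPlay it casts the mesh's anim instance to AnimBPDoorMain and caches the reference.
; Logic to toggle the anim instance's PlayerNear flag on player interaction exists but is disconnected, and the Trigger end-overlap event is empty, so this graph never changes the door state.
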(event OnComponentEndOverlap(Trigger)
  (params (OverlappedComponent :type Primitive%20Component%20Object%20Reference) (OtherActor :type Actor%20Object%20Reference) (OtherComp :type Primitive%20Component%20Object%20Reference) (OtherBodyIndex :type Integer)))

(event EventBeginPlay
  (bind _asanim_bpdoor_main (Utilities|Casting|CastToAnimBPDoorMain (Components|SkeletalMesh|GetAnimInstance (Variables|Default|GetDoor_main))))
  (Variables|Default|SetCastToDoorAnim _asanim_bpdoor_main))

(fn ConstructionScript)