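; BP_LampSwinging is a hanging lamp actor that can swing and be set lit or unlit.
; The construction script creates a dynamic bulb material instance on the skeletal mesh and sets its emission intensity from the IsOff flag.
; The SwingLight event plays the hanging light swing animation on the same mesh, looping according to the Islooping variable.
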(event Custom|SwingLight
  (Components|Animation|PlayAnimation (Variables|Default|GetSkeletalMesh) "/Game/Meshes/light/hanging_light_swing_Anim.hanging_light_swing_Anim" (Variables|Default|Getislooping)))

(fn ConstructionScript
  (|CallParentFunction)
  (bind _returnvalue (Rendering|Material|CreateDynamicMaterialInstance (Variables|Default|GetSkeletalMesh) 1 "/Game/Meshes/light/light_bulb_Inst.light_bulb_Inst" "" :!class /Script/Engine.PrimitiveComponent))
  (Variables|Default|SetMatInstance _returnvalue)
  (if (Variables|Default|GetIsOff?)
    (Rendering|Material|SetScalarParameterValue (Variables|Default|GetMatInstance) "Emission Intensity" 0.0 :!class /Script/Engine.MaterialInstanceDynamic)
    (else
      (Rendering|Material|SetScalarParameterValue (Variables|Default|GetMatInstance) "Emission Intensity" 6.0 :!class /Script/Engine.MaterialInstanceDynamic))))