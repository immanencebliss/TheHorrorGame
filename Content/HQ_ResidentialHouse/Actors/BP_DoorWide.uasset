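; Wide, lockable house door that players open and close, and that ghost interactions can slam or creak open.
; Events set PlayerNear and play rates on AnimBP_DoorWide to animate it with matching sounds, with an Engaged flag gating ghost actions.
; TimedSlam loops slams at a randomly chosen interval until SlamHammer clears the timer.
; With the PortalController initialized, Interact also force-opens the Destination door, which SwapDestination replaces for the portal puzzle.
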(event Custom|Slam%20Door
  (bind _open (Variables|Default|GetOpen))
  (bind _close (Variables|Default|GetClose))
  (bind _casttodooranim (Variables|Default|GetCastToDoorAnim))
  (if (not (Variables|Default|GetdoorLocked))
    (if (not (Variables|Default|GetEngaged))
      ;[1 1 1] Ghost Interactions
      (Variables|Default|SetEngaged true)
      (if (Variables|Default|GetDoor%20Open)
        (Variables|/Game/HQ_ResidentialHouse/Meshes/DoorWide/AnimBP_DoorWide.AnimBP_DoorWide_C|SetClosePlayRate _casttodooranim -2.0)
        (Variables|/Game/HQ_ResidentialHouse/Meshes/DoorWide/AnimBP_DoorWide.AnimBP_DoorWide_C|SetPlayerNear (Variables|Default|GetCastToDoorAnim) false)
        (Audio|Components|Audio|Play _close 0.2)
        (Variables|Default|SetDoor%20Open false)
        (Utilities|FlowControl|Delay (Variables|/Script/Engine.SoundBase|GetDuration (Variables|/Script/Engine.AudioComponent|GetSound _close)))
        (else
          (Variables|/Game/HQ_ResidentialHouse/Meshes/DoorWide/AnimBP_DoorWide.AnimBP_DoorWide_C|SetOpenPlayRate _casttodooranim 2.0)
          (Variables|/Game/HQ_ResidentialHouse/Meshes/DoorWide/AnimBP_DoorWide.AnimBP_DoorWide_C|SetPlayerNear (Variables|Default|GetCastToDoorAnim) true)
          (Audio|Components|Audio|Play _open 0.0)
          (Variables|Default|SetDoor%20Open true)
          (Utilities|FlowControl|Delay (Variables|/Script/Engine.SoundBase|GetDuration (Variables|/Script/Engine.AudioComponent|GetSound _open)))))
      (Variables|Default|SetEngaged false))))

(event Custom|Force
  (bind _casttodooranim (Variables|Default|GetCastToDoorAnim))
  ;[1 1 1] Open and closes door when player interacts with it
  (Variables|Default|SetdoorLocked false)
  (Variables|/Game/HQ_ResidentialHouse/Meshes/DoorWide/AnimBP_DoorWide.AnimBP_DoorWide_C|SetOpenPlayRate _casttodooranim 1.0)
  (Variables|/Game/HQ_ResidentialHouse/Meshes/DoorWide/AnimBP_DoorWide.AnimBP_DoorWide_C|SetClosePlayRate _casttodooranim -1.0)
  ;;[1 1 1] Open Door
  (Variables|/Game/HQ_ResidentialHouse/Meshes/DoorWide/AnimBP_DoorWide.AnimBP_DoorWide_C|SetPlayerNear (Variables|Default|GetCastToDoorAnim) true)
  (Audio|Components|Audio|Play (Variables|Default|GetOpen) 0.0)
  (Variables|Default|SetDoor%20Open true))

(event Custom|ForceClosed
  (bind _casttodooranim (Variables|Default|GetCastToDoorAnim))
  ;[1 1 1] Open and closes door when player interacts with it
  (Variables|/Game/HQ_ResidentialHouse/Meshes/DoorWide/AnimBP_DoorWide.AnimBP_DoorWide_C|SetOpenPlayRate _casttodooranim 1.0)
  (Variables|/Game/HQ_ResidentialHouse/Meshes/DoorWide/AnimBP_DoorWide.AnimBP_DoorWide_C|SetClosePlayRate _casttodooranim -1.0)
  ;;[1 1 1] Close Door
  (Variables|/Game/HQ_ResidentialHouse/Meshes/DoorWide/AnimBP_DoorWide.AnimBP_DoorWide_C|SetPlayerNear (Variables|Default|GetCastToDoorAnim) false)
  (Audio|Components|Audio|Play (Variables|Default|GetClose) 0.0)
  (Variables|Default|SetDoor%20Open false))

(event Custom|SwapDestination
  ;[1 1 1] Portal Puzzle Destination Swap
  (Variables|Default|SetDestination (Variables|Default|GetDestinationSwapper)))

(event Custom|CreakOpen
  (bind _creak (Variables|Default|GetCreak))
  (if (not (Variables|Default|GetdoorLocked))
    (if (not (Variables|Default|GetEngaged))
      ;[1 1 1] Ghost Interactions
      (Variables|Default|SetEngaged true)
      (Variables|/Game/HQ_ResidentialHouse/Meshes/DoorWide/AnimBP_DoorWide.AnimBP_DoorWide_C|SetOpenPlayRate (Variables|Default|GetCastToDoorAnim) 0.1)
      (Variables|/Game/HQ_ResidentialHouse/Meshes/DoorWide/AnimBP_DoorWide.AnimBP_DoorWide_C|SetPlayerNear (Variables|Default|GetCastToDoorAnim) true)
      (Audio|Components|Audio|Play _creak 0.0)
      (Variables|Default|SetDoor%20Open true)
      (Utilities|FlowControl|Delay (Variables|/Script/Engine.SoundBase|GetDuration (Variables|/Script/Engine.AudioComponent|GetSound _creak)))
      (Variables|Default|SetEngaged false))))

(event Custom|TimedSlam
  (bind _returnvalue (Utilities|Time|SetTimerbyEvent (delegate Custom|Slam%20Door) (Math|Random|RandomFloatinRange 0.2 1.0) true))
  (Variables|Default|SetSlamTimer _returnvalue))

(event Custom|SlamHammer
  (Utilities|Time|ClearandInvalidateTimerbyHandle (Variables|Default|GetSlamTimer)))

(event EventBeginPlay
  ;[1 1 1] Create Anim Instance Reference
  (bind _asanim_bp_door_wide (Utilities|Casting|CastToAnimBP_DoorWide (Components|SkeletalMesh|GetAnimInstance (Variables|Default|GetDoor_wide))))
  (Variables|Default|SetCastToDoorAnim _asanim_bp_door_wide))

(event EventInteract
  (params (HitComponent :type Actor%20Component%20Object%20Reference))
  (bind _casttodooranim (Variables|Default|GetCastToDoorAnim))
  (bind _destination (Variables|Default|GetDestination))
  ;[1 1 1] Open and closes door when player interacts with it
  (if (Variables|Default|GetdoorLocked)
    (Audio|PlaySoundatLocation "/Game/Blueprints/Spooks/Bathroom/DoorLocked.DoorLocked" (Transformation|GetWorldLocation (Variables|Default|GetDefaultSceneRoot)) "0, 0, 0" 1.0 1.0 0.0 0 0 0)
    (else
      (Variables|/Game/HQ_ResidentialHouse/Meshes/DoorWide/AnimBP_DoorWide.AnimBP_DoorWide_C|SetOpenPlayRate _casttodooranim 1.0)
      (Variables|/Game/HQ_ResidentialHouse/Meshes/DoorWide/AnimBP_DoorWide.AnimBP_DoorWide_C|SetClosePlayRate _casttodooranim -1.0)
      (Utilities|FlowControl|Sequence
        (:then_0
          (if (Variables|/Game/HQ_ResidentialHouse/Meshes/DoorWide/AnimBP_DoorWide.AnimBP_DoorWide_C|GetPlayerNear (Variables|Default|GetCastToDoorAnim))
            ;;[1 1 1] Close Door
            (Variables|/Game/HQ_ResidentialHouse/Meshes/DoorWide/AnimBP_DoorWide.AnimBP_DoorWide_C|SetPlayerNear (Variables|Default|GetCastToDoorAnim) false)
            (Audio|Components|Audio|Play (Variables|Default|GetClose) 0.0)
            (Variables|Default|SetDoor%20Open false)
            (else
              ;;[1 1 1] Open Door
              (Variables|/Game/HQ_ResidentialHouse/Meshes/DoorWide/AnimBP_DoorWide.AnimBP_DoorWide_C|SetPlayerNear (Variables|Default|GetCastToDoorAnim) true)
              (Audio|Components|Audio|Play (Variables|Default|GetOpen) 0.0)
              (Variables|Default|SetDoor%20Open true))))
        (:then_1
          (if (Variables|/Game/Blueprints/PortalController.PortalController_C|GetInitialized? (Variables|Default|GetPortalController))
            (Utilities|IsValid _destination
              (:Is%20Valid
                (CallFunction|Force _destination)))))))))

(fn ConstructionScript)