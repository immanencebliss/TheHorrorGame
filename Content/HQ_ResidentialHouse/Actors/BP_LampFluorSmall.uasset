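; Small fluorescent lamp actor for the residential house, a switchable light built on a parent class with its own ToggleLight.
; The construction script caches the first rect light's intensity and gives each static mesh a dynamic material instance in slot 0.
; IsOff sets both rect light visibility and material emission at construction, so the glow matches the light.
; ToggleLight flips the RectLight's visibility, then calls the parent implementation.
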(event EventToggleLight
  (Rendering|ToggleVisibility (Variables|Default|GetRectLight) false)
  (|CallParentFunction))

(fn ConstructionScript
  (Utilities|FlowControl|Sequence
    (:then_0
      (bind _output_get (Variables|Default|SetRects (Actor|GetComponentsByClass "/Script/Engine.RectLightComponent")))
      (Variables|Default|SetDefault%20intensity (Variables|/Script/Engine.LightComponentBase|GetIntensity (Utilities|Array|Get(acopy) _output_get))))
    (:then_1
      (bind _output_get_2 (Variables|Default|Setmeshes (Actor|GetComponentsByClass "/Script/Engine.StaticMeshComponent")))
      (for _array_element _output_get_2
        (bind _returnvalue (Rendering|Material|CreateDynamicMaterialInstance _array_element 0 (Rendering|Material|GetMaterial _array_element 0) "None" :!class /Script/Engine.PrimitiveComponent))
        (Variables|Default|SetMatInstance _returnvalue)
        (for _array_element_2 (Variables|Default|GetRects)
          (if (Variables|Default|GetIsOff?)
            (Rendering|SetVisibility _array_element_2 false false)
            (Rendering|Material|SetScalarParameterValue (Variables|Default|GetMatInstance) "Emission Intensity" 0.0 :!class /Script/Engine.MaterialInstanceDynamic)
            (else
              (Rendering|SetVisibility _array_element_2 true false)
              (Rendering|Material|SetScalarParameterValue (Variables|Default|GetMatInstance) "Emission Intensity" 15.0 :!class /Script/Engine.MaterialInstanceDynamic))))))))