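; Baby is an interactable prop that triggers the game's ending.
; Interact blends the view to a camera, plays the Finale level sequence, then uses timed delays to slam or creak open a door and flicker a light.
; It then sets the Alpha parameter on a dynamic material created in the construction script and quits the game after a final pause.
; A separate event activates its audio.
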(event Custom|Activate%20audio
  (Components|Activation|Activate (Variables|Default|GetAudio) false))

(event EventInteract
  (params (HitComponent :type Actor%20Component%20Object%20Reference))
  (bind _door (Variables|Default|GetDoor))
  (Game|Player|SetViewTargetwithBlend (Game|GetPlayerController 0) (Variables|Default|GetCamera) 1.0 "VTBlend_Linear" 0.0 false)
  (Utilities|FlowControl|Delay 1.0)
  (bind _returnvalue (Sequencer|Player|CreateLevelSequencePlayer "/Game/Finale.Finale"))
  (Sequencer|Player|Play _returnvalue :!class /Script/MovieScene.MovieSceneSequencePlayer)
  (Utilities|FlowControl|Delay 13.0)
  (if (Variables|/Game/HQ_ResidentialHouse/Actors/BP_DoorWide.BP_DoorWide_C|GetDoor%20Open _door)
    (Default|SlamDoor _door)
    (else
      (Default|CreakOpen _door)))
  (Utilities|FlowControl|Delay 1.0)
  (Default|IFlickerShort (Variables|Default|GetLight) false)
  (Utilities|FlowControl|Delay 3.7)
  (Rendering|Material|SetScalarParameterValue (Variables|Default|GetMatInst) "Alpha" 1.0 :!class /Script/Engine.MaterialInstanceDynamic)
  (Utilities|FlowControl|Delay 0.2)
  (Utilities|FlowControl|Delay 1e+01)
  (Game|QuitGame 0 "Quit"))

(fn ConstructionScript
  (bind _staticmesh (Variables|Default|GetStaticMesh))
  (|CallParentFunction)
  (bind _returnvalue (Rendering|Material|CreateDynamicMaterialInstance _staticmesh 0 (Rendering|Material|GetMaterial _staticmesh 0) "None" :!class /Script/Engine.PrimitiveComponent))
  (Variables|Default|SetMatInst _returnvalue))