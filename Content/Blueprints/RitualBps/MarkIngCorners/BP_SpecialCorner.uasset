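; BP_SpecialCorner is a trigger for the corner-marking ritual puzzle that tells the phone UI when the player stands in a special corner.
; On overlap, it checks that the puzzle is initialized and its RoomToMark matches the game mode's current MarkingOrder entry, then sets SpecialCorner on the first WID_CellPhoneMaster widget found.
; Leaving clears the flag while the puzzle is initialized, without rechecking the room.
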(event OnComponentBeginOverlap(overlapper)
  (params (OverlappedComponent :type Primitive%20Component%20Object%20Reference) (OtherActor :type Actor%20Object%20Reference) (OtherComp :type Primitive%20Component%20Object%20Reference) (OtherBodyIndex :type Integer) (bFromSweep :type Boolean) (SweepResult :type Hit%20Result%20Structure%20%28by%20ref%29))
  (bind _returnvalue (Game|GetGameMode))
  (bind _asthird_person_game_mode (Utilities|Casting|CastToThirdPersonGameMode _returnvalue))
  (if (Math|Boolean|ANDBoolean (Actor|ActorHasTag OtherActor "player") (Utilities|Enum|Equal(Enum) (Variables|Default|GetRoomToMark) (Utilities|Array|Get(acopy) (Variables|/Game/ThirdPersonBP/Blueprints/ThirdPersonGameMode.ThirdPersonGameMode_C|GetMarkingOrder _asthird_person_game_mode) (Variables|/Game/ThirdPersonBP/Blueprints/ThirdPersonGameMode.ThirdPersonGameMode_C|GetCurrentRoomToMark _asthird_person_game_mode))) (Variables|/Game/ThirdPersonBP/Blueprints/ThirdPersonGameMode.ThirdPersonGameMode_C|GetMarkingPuzzleInitialized _asthird_person_game_mode))
    (bind _foundwidgets (Widget|GetAllWidgetsOfClass "/Game/Blueprints/Cellphone/WID_CellPhoneMaster.WID_CellPhoneMaster_C" false))
    (Variables|/Game/Blueprints/Cellphone/WID_CellPhoneMaster.WID_CellPhoneMaster_C|SetSpecialCorner? (Utilities|Array|Get(acopy) _foundwidgets) true)))

(event OnComponentEndOverlap(overlapper)
  (params (OverlappedComponent :type Primitive%20Component%20Object%20Reference) (OtherActor :type Actor%20Object%20Reference) (OtherComp :type Primitive%20Component%20Object%20Reference) (OtherBodyIndex :type Integer))
  (if (and (Actor|ActorHasTag OtherActor "player") (Variables|/Game/ThirdPersonBP/Blueprints/ThirdPersonGameMode.ThirdPersonGameMode_C|GetMarkingPuzzleInitialized (.AsThird%20Person%20Game%20Mode (Utilities|Casting|CastToThirdPersonGameMode (Game|GetGameMode)))))
    (bind _foundwidgets (Widget|GetAllWidgetsOfClass "/Game/Blueprints/Cellphone/WID_CellPhoneMaster.WID_CellPhoneMaster_C" false))
    (Variables|/Game/Blueprints/Cellphone/WID_CellPhoneMaster.WID_CellPhoneMaster_C|SetSpecialCorner? (Utilities|Array|Get(acopy) _foundwidgets) false)))

(event EventBeginPlay
  (bind _asthird_person_game_mode (Utilities|Casting|CastToThirdPersonGameMode (Game|GetGameMode)))
  (Variables|Default|SetGameMode _asthird_person_game_mode))

(event Collision|EventActorBeginOverlap
  (params (OtherActor :type Actor%20Object%20Reference)))

(event EventTick
  (params (DeltaSeconds :type Float%20%28single-precision%29)))

(fn ConstructionScript)