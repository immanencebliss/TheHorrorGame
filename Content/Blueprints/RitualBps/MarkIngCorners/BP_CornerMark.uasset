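; BP_CornerMark is a ritual corner marker that shows a magic circle symbol on a plane, chosen by a word.
; The construction script creates and stores a dynamic material instance on the plane, which is hidden at BeginPlay.
; SetMatieral maps each of four words to its own circle texture, sets it as the material's symbol parameter and makes the plane visible.
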(event EventBeginPlay
  (Rendering|SetVisibility (Variables|Default|GetPlane) false false))

(event Collision|EventActorBeginOverlap
  (params (OtherActor :type Actor%20Object%20Reference)))

(event EventTick
  (params (DeltaSeconds :type Float%20%28single-precision%29)))

(fn ConstructionScript
  (bind _returnvalue (Rendering|Material|CreateDynamicMaterialInstance (Variables|Default|GetPlane) 0 "/Game/Blueprints/RitualBps/MarkIngCorners/MAT_CornerMark_Inst.MAT_CornerMark_Inst" "None" :!class /Script/Engine.PrimitiveComponent))
  (Variables|Default|SetCornerTexture _returnvalue))

(fn SetMatieral
  (params (word :type String))
  (switch string word
    (:jimmy
      (Rendering|Material|SetTextureParameterValue (Variables|Default|GetCornerTexture) "symbol" "/Game/MagicCircle14.MagicCircle14"))
    (:hocus
      (Rendering|Material|SetTextureParameterValue (Variables|Default|GetCornerTexture) "symbol" "/Game/MagicCircle13.MagicCircle13"))
    (:pocus
      (Rendering|Material|SetTextureParameterValue (Variables|Default|GetCornerTexture) "symbol" "/Game/MagicCircle11.MagicCircle11"))
    (:fuck
      (Rendering|Material|SetTextureParameterValue (Variables|Default|GetCornerTexture) "symbol" "/Game/MagicCircle10.MagicCircle10")))
  (Rendering|SetVisibility (Variables|Default|GetPlane) true false))