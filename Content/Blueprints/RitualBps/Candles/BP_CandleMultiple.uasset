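; Interactable cluster of three candles, one main and two small, that toggles between lit and unlit.
; Interact flips CandleOn, showing or hiding the three flame proxies and the shared FlameLight, with TurnOffCandle handling the off state.
; The construction script applies the initial lit state and positions the candles in one of four preset layouts chosen by Arrangment.
; A timeline started on BeginPlay varies the light's intensity within a narrow range.
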(event EventBeginPlay
  ;[1 1 1] Sets Flame To off by default
  (bind _alpha (Timeline|Timeline_0 Play)
    (:Update
      (Rendering|Components|Light|SetIntensity (Variables|Default|GetFlameLight) (Math|Float|Lerp 0.25 0.15 _alpha)))))

(event EventInteract
  (params (HitComponent :type Actor%20Component%20Object%20Reference))
  ;[1 1 1] Toggle if candle is on or not
  (if (Variables|Default|GetCandleOn?)
    (Variables|Default|SetCandleOn? false)
    (CallFunction|TurnOffCandle)
    (else
      (Variables|Default|SetCandleOn? true)
      (Rendering|SetVisibility (Variables|Default|GetFlameProxy) true false)
      (Rendering|SetVisibility (Variables|Default|GetFlameLight) true false))))

(fn ConstructionScript
  (if (Variables|Default|GetCandleOn?)
    (Rendering|SetVisibility (Variables|Default|GetFlameLight) true false)
    (Rendering|SetVisibility (Variables|Default|GetFlameProxy) true false)
    (else
      (Rendering|SetVisibility (Variables|Default|GetFlameLight) false false)
      (Rendering|SetVisibility (Variables|Default|GetFlameProxy) false false)))
  (switch int (Variables|Components|GetArrangment)
    (:0
      (Transformation|SetRelativeLocation (Variables|Default|GetCandle) "0, 0, 0" false false)
      (Transformation|SetRelativeLocation (Variables|Default|GetSmallCandle) "6.865482, 0,0.000000" false false)
      (Transformation|SetRelativeLocation (Variables|Default|GetSmallCandle2) "3.079077,6.170180,0.000000" false false))
    (:1
      (Transformation|SetRelativeLocation (Variables|Default|GetCandle) "0, 0, 0" false false)
      (Transformation|SetRelativeLocation (Variables|Default|GetSmallCandle) "-2.716128,-8.332912,0.000000" false false)
      (Transformation|SetRelativeLocation (Variables|Default|GetSmallCandle2) "-2.772741,7.498804,0.000000" false false))
    (:2
      (Transformation|SetRelativeLocation (Variables|Default|GetCandle) "0, 0, 0" false false)
      (Transformation|SetRelativeLocation (Variables|Default|GetSmallCandle) "7.148779,12.870733,0.000000" false false)
      (Transformation|SetRelativeLocation (Variables|Default|GetSmallCandle2) "4.237351,-2.643579,0.000000" false false))
    (:3
      (Transformation|SetRelativeLocation (Variables|Default|GetCandle) "0, 0, 0" false false)
      (Transformation|SetRelativeLocation (Variables|Default|GetSmallCandle) "-15.887152,-15.742151,0.000000" false false)
      (Transformation|SetRelativeLocation (Variables|Default|GetSmallCandle2) "8.687374,13.794287,0.000000" false false))))

(fn TurnOffCandle
  (Variables|Default|SetCandleOn? false)
  (Rendering|SetVisibility (Variables|Default|GetFlameProxy) false false)
  (Rendering|SetVisibility (Variables|Default|GetFlameLight) false false))