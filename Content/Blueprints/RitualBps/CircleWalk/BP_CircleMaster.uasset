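; BP_CircleMaster tracks progress as numbered points of a circle are passed in sequence, apparently for a circle-walk ritual.
; CirclePointCheck accepts any point as the start, then expects ascending numbers, wrapping to the first after an expected last point.
; Each correct point raises a passed count capped at the total, while a wrong one clears it and stops the circle.
; The event graph is empty, and nothing here acts on completion.
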(event EventBeginPlay)

(event Collision|EventActorBeginOverlap
  (params (OtherActor :type Actor%20Object%20Reference)))

(event EventTick
  (params (DeltaSeconds :type Float%20%28single-precision%29)))

(fn ConstructionScript)

(fn CirclePointCheck
  (params (CirclePoint :type Integer))
  (Variables|Default|SetCurrentCirclePoint CirclePoint)
  (if (Variables|Default|GetCircleStarted?)
    (if (== (Variables|Default|GetCurrentCirclePoint) (Variables|Default|GetExpectedCirclePoint))
      (Math|Integer|IncrementInt (Variables|Default|GetExpectedCirclePoint)
        (:%20%20
          (if (> (Variables|Default|GetExpectedCirclePoint) (Variables|Default|GetTotalCirclePoints))
            (Variables|Default|SetExpectedCirclePoint 1))
          (if (not (>= (Variables|Default|GetNumber%20Of%20Circle%20Points%20Passed) (Variables|Default|GetTotalCirclePoints)))
            (Math|Integer|IncrementInt (Variables|Default|GetNumber%20Of%20Circle%20Points%20Passed)))))
      (else
        (Variables|Default|SetCircleStarted? false)
        (Variables|Default|SetNumber%20Of%20Circle%20Points%20Passed 0)))
    (else
      (bind _result (Math|Integer|IncrementInt (Variables|Default|GetCurrentCirclePoint))
        (:%20%20
          (Variables|Default|SetExpectedCirclePoint _result)
          (Math|Integer|IncrementInt (Variables|Default|GetNumber%20Of%20Circle%20Points%20Passed)
            (:%20%20
              (Variables|Default|SetCircleStarted? true))))))))