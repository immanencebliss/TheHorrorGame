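; Master actor for the circle-walk ritual puzzle, which tracks circle points hit in sequence and glows brighter as progress builds.
; CirclePointCheck accepts any starting point, expects wrapping consecutive order, resets on a mistake, and on completion flags ThirdPersonGameMode and calls LightUpCircle.
; Timelines lerp dynamic material brightness and visibility by increments derived from the point count, with inner detail joining from the third point.
; The final flash logic is unwired.
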(event Custom|CircleMatieralTimeLine
  (bind _basecircle (Timeline|CircleVisibility Play)
    (:Update
      (Rendering|Material|SetScalarParameterValue (Variables|Default|GetBaseCircleMat) "Brightness" (Math|Float|Lerp (Variables|LerpValues|GetCurrentPositionBrightness) (Variables|LerpValues|GetTargetPositionBrightness) _basecircle) :!class /Script/Engine.MaterialInstanceDynamic)
      (Rendering|Material|SetScalarParameterValue (Variables|Default|GetBaseCircleMat) "Visibility" (Math|Float|Lerp (Variables|LerpValues|GetCurrentPositionVisibility) (Variables|LerpValues|GetTargetPositionvisibility) _basecircle) :!class /Script/Engine.MaterialInstanceDynamic))
    (:Finished
      (CallFunction|SetCurrentVisandBright))))

(event Custom|DetailCircleTimeLine
  (bind _detaillerp (Timeline|DetailCircleVisibility Play)
    (:Update
      (Rendering|Material|SetScalarParameterValueonMaterials (Variables|Default|GetCircleInnerDetail) "Brightness" (Math|Float|Lerp (Variables|LerpValuesDetail|GetCurrentPositionBrightnessDetail) (Variables|LerpValuesDetail|GetTargetPositionBrightnessDetail) _detaillerp))
      (Rendering|Material|SetScalarParameterValueonMaterials (Variables|Default|GetCircleInnerDetail) "Visibility" (Math|Float|Lerp (Variables|LerpValuesDetail|GetCurrentPositionVisibilityDetail) (Variables|LerpValuesDetail|GetTargetPositionVisibilityDetail) _detaillerp)))
    (:Finished
      (CallFunction|SetCurrentVisandBrightDetail))))

(event Custom|Final%20Flash)

(event Collision|EventActorBeginOverlap
  (params (OtherActor :type Actor%20Object%20Reference)))

(event EventTick
  (params (DeltaSeconds :type Float%20%28single-precision%29)))

(event EventBeginPlay
  (Rendering|SetVisibility (Variables|Default|GetBaseCircle) false false)
  (Rendering|SetVisibility (Variables|Default|GetCircleInnerDetail) false false)
  (CallFunction|CalculateLerpAmounts)
  (Rendering|Material|SetScalarParameterValueonMaterials (Variables|Default|GetCircleInnerDetail) "Visibility" 0.0)
  (Rendering|Material|SetScalarParameterValue (Variables|Default|GetBaseCircleMat) "Visibility" 0.0 :!class /Script/Engine.MaterialInstanceDynamic))

(fn ConstructionScript
  (bind _returnvalue (Rendering|Material|CreateDynamicMaterialInstance (Variables|Default|GetBaseCircle) 0 "/Game/Blueprints/RitualBps/CircleWalk/MATINST_RitualCircleBase.MATINST_RitualCircleBase" "None" :!class /Script/Engine.PrimitiveComponent))
  (Variables|Default|SetBaseCircleMat _returnvalue)
  (bind _returnvalue_2 (Rendering|Material|CreateDynamicMaterialInstance (Variables|Default|GetCircleInnerDetail) 0 "/Game/Blueprints/RitualBps/CircleWalk/MATINST_RitualCircleDetails.MATINST_RitualCircleDetails" "None" :!class /Script/Engine.PrimitiveComponent))
  (Variables|Default|SetDetailCircleMat _returnvalue_2))

(fn CirclePointCheck
  (params (CirclePoint :type Integer))
  (if (not (Variables|Default|GetFinished?))
    (Variables|Default|SetCurrentCirclePoint CirclePoint)
    (if (Variables|Default|GetCircleStarted?)
      (if (== (Variables|Default|GetCurrentCirclePoint) (Variables|Default|GetExpectedCirclePoint))
        (Math|Integer|IncrementInt (Variables|Default|GetExpectedCirclePoint)
          (:%20%20
            (if (> (Variables|Default|GetExpectedCirclePoint) (- (Math|Float|Truncate (Variables|Default|GetTotalCirclePoints)) 1))
              (Variables|Default|SetExpectedCirclePoint 1))
            (if (>= (Variables|Default|GetNumber%20Of%20Circle%20Points%20Passed) (Math|Float|Truncate (Variables|Default|GetTotalCirclePoints)))
              (Variables|Default|SetFinished? true)
              (bind _asthird_person_game_mode (Utilities|Casting|CastToThirdPersonGameMode (Game|GetGameMode)))
              (Variables|/Game/ThirdPersonBP/Blueprints/ThirdPersonGameMode.ThirdPersonGameMode_C|SetCirclePuzzleComplete _asthird_person_game_mode true)
              (Default|LightUpCircle _asthird_person_game_mode "NewEnumerator2")
              (else
                (Math|Integer|IncrementInt (Variables|Default|GetNumber%20Of%20Circle%20Points%20Passed)
                  (:%20%20
                    (if (>= (Variables|Default|GetNumber%20Of%20Circle%20Points%20Passed) 3)
                      (Variables|LerpValuesDetail|SetTargetPositionBrightnessDetail (+ (Variables|LerpValuesDetail|GetTargetPositionBrightnessDetail) (Variables|LerpValuesDetail|GetBrightnessToAddDetail)))
                      (Variables|LerpValuesDetail|SetTargetPositionVisibilityDetail (+ (Variables|LerpValuesDetail|GetTargetPositionVisibilityDetail) (Variables|LerpValuesDetail|GetVisibilityToDetail)))
                      (CallFunction|DetailCircleTimeLine))
                    (Variables|LerpValues|SetTargetPositionBrightness (+ (Variables|LerpValues|GetTargetPositionBrightness) (Variables|LerpValues|GetBrightnessToAdd)))
                    (Variables|LerpValues|SetTargetPositionvisibility (+ (Variables|LerpValues|GetTargetPositionvisibility) (Variables|LerpValues|GetVisibilityToAdd)))
                    (CallFunction|CircleMatieralTimeLine)))))))
        (else
          (CallFunction|Resetcircle)))
      (else
        (bind _result (Math|Integer|IncrementInt (Variables|Default|GetCurrentCirclePoint))
          (:%20%20
            (Variables|Default|SetExpectedCirclePoint _result)
            (Math|Integer|IncrementInt (Variables|Default|GetNumber%20Of%20Circle%20Points%20Passed)
              (:%20%20
                (Variables|Default|SetCircleStarted? true)
                (Rendering|SetVisibility (Variables|Default|GetBaseCircle) true false)
                (Rendering|SetVisibility (Variables|Default|GetCircleInnerDetail) true false)))))))))

(fn CalculateLerpAmounts
  (bind _totalcirclepoints (Variables|Default|GetTotalCirclePoints))
  (bind _returnvalue (- _totalcirclepoints 1.0))
  (bind _returnvalue_2 (- _totalcirclepoints 4.0))
  (Utilities|FlowControl|Sequence
    (:then_0
      (Variables|LerpValues|SetBrightnessToAdd (/ 6.0 _returnvalue))
      (Variables|LerpValues|SetVisibilityToAdd (/ 1.0 _returnvalue))
      (Variables|LerpValuesDetail|SetBrightnessToAddDetail (/ 6.0 _returnvalue_2))
      (Variables|LerpValuesDetail|SetVisibilityToDetail (/ 1.0 _returnvalue_2)))))

(fn SetCurrentVisandBright
  (Variables|LerpValues|SetCurrentPositionBrightness (+ (Variables|LerpValues|GetCurrentPositionBrightness) (Variables|LerpValues|GetBrightnessToAdd)))
  (Variables|LerpValues|SetCurrentPositionVisibility (+ (Variables|LerpValues|GetCurrentPositionVisibility) (Variables|LerpValues|GetVisibilityToAdd))))

(fn Resetcircle
  (Utilities|FlowControl|Sequence
    (:then_0
      (Variables|Default|SetCircleStarted? false)
      (Variables|Default|SetNumber%20Of%20Circle%20Points%20Passed 0))
    (:then_1
      (Variables|LerpValues|SetCurrentPositionBrightness 0.0)
      (Variables|LerpValues|SetTargetPositionBrightness (Variables|LerpValues|GetBrightnessToAdd))
      (Variables|LerpValues|SetCurrentPositionVisibility 0.0)
      (Variables|LerpValues|SetTargetPositionvisibility (Variables|LerpValues|GetVisibilityToAdd)))
    (:then_2
      (Variables|LerpValuesDetail|SetCurrentPositionBrightnessDetail 0.0)
      (Variables|LerpValuesDetail|SetTargetPositionBrightnessDetail (Variables|LerpValuesDetail|GetBrightnessToAddDetail))
      (Variables|LerpValuesDetail|SetCurrentPositionVisibilityDetail 0.0)
      (Variables|LerpValuesDetail|SetTargetPositionVisibilityDetail (Variables|LerpValuesDetail|GetVisibilityToDetail)))
    (:then_3
      (Rendering|SetVisibility (Variables|Default|GetBaseCircle) false false)
      (Rendering|Material|SetScalarParameterValue (Variables|Default|GetBaseCircleMat) "Brightness" 0.0 :!class /Script/Engine.MaterialInstanceDynamic)
      (Rendering|Material|SetScalarParameterValue (Variables|Default|GetBaseCircleMat) "Visibility" 0.0 :!class /Script/Engine.MaterialInstanceDynamic))
    (:then_4
      (Rendering|SetVisibility (Variables|Default|GetCircleInnerDetail) false false)
      (Rendering|Material|SetScalarParameterValue (Variables|Default|GetDetailCircleMat) "Brightness" 0.0 :!class /Script/Engine.MaterialInstanceDynamic)
      (Rendering|Material|SetScalarParameterValue (Variables|Default|GetDetailCircleMat) "Visibility" 0.0 :!class /Script/Engine.MaterialInstanceDynamic))))

(fn SetCurrentVisandBrightDetail
  (Variables|LerpValuesDetail|SetCurrentPositionBrightnessDetail (+ (Variables|LerpValuesDetail|GetCurrentPositionBrightnessDetail) (Variables|LerpValuesDetail|GetBrightnessToAddDetail)))
  (Variables|LerpValuesDetail|SetCurrentPositionVisibilityDetail (+ (Variables|LerpValuesDetail|GetCurrentPositionVisibilityDetail) (Variables|LerpValuesDetail|GetVisibilityToDetail))))