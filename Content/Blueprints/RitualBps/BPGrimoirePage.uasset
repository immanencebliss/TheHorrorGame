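; BPGrimoirePage is a collectible grimoire page that glows and materializes on BeginPlay using timelines driving a point light and a dissolve material parameter.
; Interact plays a paper sound, notifies the UI, activates the page set by SetPage in the Grimoire widget, then destroys the actor.
; It also increments the game mode's pickup count and runs GateCheck.
; DisolveOut lerps dissolve between identical values, and a marking-puzzle flag branch is unconnected.
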(event Custom|DisolveOut
  (bind _dissolving (Timeline|fadeout Play)
    (:Update
      (Rendering|Material|SetScalarParameterValue (Variables|Default|GetGrimoireMAT) "dissolve" (Math|Float|Lerp 0.0 0.0 _dissolving) :!class /Script/Engine.MaterialInstanceDynamic))
    (:Finished
      (Actor|DestroyActor))))

(event Custom|dissolveIn
  (bind _dissolving (Timeline|Matieralize Play)
    (:Update
      (Rendering|Material|SetScalarParameterValue (Variables|Default|GetGrimoireMAT) "dissolve" (Math|Float|Lerp 0.0 1.0 _dissolving) :!class /Script/Engine.MaterialInstanceDynamic))))

(event EventBeginPlay
  (bind _alpha (Timeline|Glow Play)
    (:Update
      (Rendering|Components|Light|SetIntensity (Variables|Default|GetPointLight) (Math|Float|Lerp (Variables|Default|GetLowInt) (Variables|Default|GetHighInt) _alpha))
      (CallFunction|Dissolvein))))

(event EventInteract
  (params (HitComponent :type Actor%20Component%20Object%20Reference))
  (bind _returnvalue (Game|GetGameMode))
  (bind _asthird_person_game_mode (Utilities|Casting|CastToThirdPersonGameMode _returnvalue))
  (Audio|PlaySoundatLocation "/Game/Audio/paper_scrunch.paper_scrunch" (Transformation|GetWorldLocation (Variables|Default|GetPage)) "0, 0, 0" 1.0 1.0 0.0 0 0 0)
  (bind _foundwidgets (Widget|GetAllWidgetsOfClass "/Game/Blueprints/RitualBps/UI_notification.UI_notification_C" false))
  (Default|NotifyOfGrimoire (Utilities|Array|Get(acopy) _foundwidgets))
  (bind _foundwidgets_2 (Widget|GetAllWidgetsOfClass "/Game/UI/Grimoire.Grimoire_C" false))
  (bind _output_get (Variables|Default|SetcastGrimoire (Utilities|Array|Get(acopy) _foundwidgets_2)))
  (Default|ActivatePage _output_get (Variables|Default|GetPageindex) (Variables|Default|GetLeftPage))
  (Math|Integer|IncrementInt (Variables|/Game/ThirdPersonBP/Blueprints/ThirdPersonGameMode.ThirdPersonGameMode_C|GetPagesPickedUp _asthird_person_game_mode)
    (:%20%20
      (Default|GateCheck _asthird_person_game_mode)
      (Actor|DestroyActor))))

(fn ConstructionScript
  (bind _returnvalue (Rendering|Material|CreateDynamicMaterialInstance (Variables|Default|GetPage) 0 "/Game/Blueprints/RitualBps/MAT_GrimoirePage_Inst.MAT_GrimoirePage_Inst" "None" :!class /Script/Engine.PrimitiveComponent))
  (Variables|Default|SetGrimoireMAT _returnvalue))

(fn SetPage
  (params (LeftPage? :type Boolean) (Index :type Integer))
  (Variables|Default|SetLeftPage LeftPage?)
  (Variables|Default|SetPageindex Index))