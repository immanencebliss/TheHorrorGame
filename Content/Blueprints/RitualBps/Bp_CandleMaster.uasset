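; Candle puzzle master Blueprint for the ritual, tracking which candles are lit and whether the puzzle is solved.
; CheckCandleLit records each lit candle and counts correct ones toward a required amount, printing a debug success message when reached.
; A wrong candle resets the count, turns off every recorded candle and clears the list.
; Its event graph and construction script are empty, so all logic runs through that one function.
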(event EventBeginPlay)

(event Collision|EventActorBeginOverlap
  (params (OtherActor :type Actor%20Object%20Reference)))

(event EventTick
  (params (DeltaSeconds :type Float%20%28single-precision%29)))

(fn ConstructionScript)

(fn CheckCandleLit
  (params (CorrectCandlle :type Boolean) (CandleLit :type BP%20Candle%20Object%20Reference))
  ;[1 1 1] Stores a reference to the candle being lit
  (Utilities|Array|Add (Variables|Default|GetCandlesLit) CandleLit)
  (if CorrectCandlle
    ;[1 1 1] If the correct candle is being lit add one to the amount lit and check if the amount needed has been reached
    (Math|Integer|IncrementInt (Variables|Default|GetAmount%20Of%20CandlesLit)
      (:%20%20
        (if (>= (Variables|Default|GetAmount%20Of%20CandlesLit) (Variables|Default|GetAmount%20Of%20Candles%20Needed))
          (Development|PrintString "YOU did it"))))
    (else
      ;[1 1 1] If the wrong candle is lit set candle lit to 0, turn off all the lit candles and clear the references
      (Variables|Default|SetAmount%20Of%20CandlesLit 0)
      (for _array_element (Variables|Default|GetCandlesLit)
        (Default|TurnOffCandle _array_element))
      (Utilities|Array|Clear (Variables|Default|GetCandlesLit)))))