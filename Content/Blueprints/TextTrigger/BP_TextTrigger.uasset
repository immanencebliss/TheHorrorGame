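; BP_TextTrigger is a placeable trigger that sends a scripted phone text when the player reaches a story location.
; On overlap by an actor tagged "player", it switches on its Text setting to pick the message for that location.
; It finds the WID_CellPhoneMaster widget, calls ScriptedText with the matching key, then destroys itself.
; The first-portal message fires only once the PortalController is initialized.
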(event OnComponentBeginOverlap(TextTrigger)
  (params (OverlappedComponent :type Primitive%20Component%20Object%20Reference) (OtherActor :type Actor%20Object%20Reference) (OtherComp :type Primitive%20Component%20Object%20Reference) (OtherBodyIndex :type Integer) (bFromSweep :type Boolean) (SweepResult :type Hit%20Result%20Structure%20%28by%20ref%29))
  (if (Actor|ActorHasTag OtherActor "player")
    (switch Utilities|FlowControl|Switch|SwitchonENU_TextTriggers (Variables|Default|GetText)
      (:NewEnumerator0
        (Utilities|FlowControl|DoOnce false
          (:Completed
            (bind _foundwidgets (Widget|GetAllWidgetsOfClass "/Game/Blueprints/Cellphone/WID_CellPhoneMaster.WID_CellPhoneMaster_C" false))
            (Default|ScriptedText (Utilities|Array|Get(acopy) _foundwidgets) "livingroom")
            (Actor|DestroyActor :!label _label))))
      (:NewEnumerator1
        (Utilities|FlowControl|DoOnce false
          (:Completed
            (bind _foundwidgets_2 (Widget|GetAllWidgetsOfClass "/Game/Blueprints/Cellphone/WID_CellPhoneMaster.WID_CellPhoneMaster_C" false))
            (Default|ScriptedText (Utilities|Array|Get(acopy) _foundwidgets_2) "upstairs")
            (goto _label))))
      (:NewEnumerator2
        (if (Variables|/Game/Blueprints/PortalController.PortalController_C|GetInitialized? (Variables|Default|GetPortalController))
          (Utilities|FlowControl|DoOnce false
            (:Completed
              (bind _foundwidgets_3 (Widget|GetAllWidgetsOfClass "/Game/Blueprints/Cellphone/WID_CellPhoneMaster.WID_CellPhoneMaster_C" false))
              (Default|ScriptedText (Utilities|Array|Get(acopy) _foundwidgets_3) "portal")
              (goto _label)))))
      (:NewEnumerator3
        (Utilities|FlowControl|DoOnce false
          (:Completed
            (bind _foundwidgets_4 (Widget|GetAllWidgetsOfClass "/Game/Blueprints/Cellphone/WID_CellPhoneMaster.WID_CellPhoneMaster_C" false))
            (Default|ScriptedText (Utilities|Array|Get(acopy) _foundwidgets_4) "bridge")
            (goto _label)))))))

(event EventBeginPlay)

(event Collision|EventActorBeginOverlap
  (params (OtherActor :type Actor%20Object%20Reference)))

(event EventTick
  (params (DeltaSeconds :type Float%20%28single-precision%29)))

(fn ConstructionScript)