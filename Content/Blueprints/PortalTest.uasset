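; Portal actor, paired with a Destination portal, that teleports the player character between the two and drives a render-target view through the link.
; Each tick it places the Destination's PortalView capture at the player camera's transform mapped between the portals with a 180-degree yaw flip.
; Overlapping the hidden Plane moves the player to the Destination and copies that view's rotation, disabling the exit's teleport until overlap ends to prevent bouncing back.
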(event OnComponentBeginOverlap(Plane)
  (params (OverlappedComponent :type Primitive%20Component%20Object%20Reference) (OtherActor :type Actor%20Object%20Reference) (OtherComp :type Primitive%20Component%20Object%20Reference) (OtherBodyIndex :type Integer) (bFromSweep :type Boolean) (SweepResult :type Hit%20Result%20Structure%20%28by%20ref%29))
  (bind _destination (Variables|Default|GetDestination))
  (if (== OtherActor (Game|GetPlayerCharacter 0))
    (if (Variables|Default|GetCanTeleport)
      (Variables|/Game/Blueprints/Portal.Portal_C|SetCanTeleport _destination false)
      (Transformation|SetActorLocation OtherActor (Transformation|GetWorldLocation (Variables|/Game/Blueprints/Portal.Portal_C|GetDefaultSceneRoot _destination)) false false)
      (Pawn|SetControlRotation (Game|GetPlayerController 0) (Transformation|GetWorldRotation (Variables|/Game/Blueprints/Portal.Portal_C|GetPortalView _destination))))))

(event OnComponentEndOverlap(Plane)
  (params (OverlappedComponent :type Primitive%20Component%20Object%20Reference) (OtherActor :type Actor%20Object%20Reference) (OtherComp :type Primitive%20Component%20Object%20Reference) (OtherBodyIndex :type Integer))
  (Variables|Default|SetCanTeleport true))

(event Custom|Initialize
  (Rendering|SetVisibility (Variables|Default|GetPlane) false false)
  (Collision|SetCollisionEnabled (Variables|Default|GetPlane) "QueryOnly"))

(event EventTick
  (params (DeltaSeconds :type Float%20%28single-precision%29))
  (bind _returnvalue (Game|GetPlayerController 0))
  (bind _defaultsceneroot (Variables|Default|GetDefaultSceneRoot))
  (bind _destination (Variables|Default|GetDestination))
  (bind _returnvalue_2 (Transformation|GetWorldRotation _defaultsceneroot))
  (bind _defaultsceneroot_2 (Variables|/Game/Blueprints/Portal.Portal_C|GetDefaultSceneRoot _destination))
  (bind _playercameramanager (Variables|/Script/Engine.PlayerController|GetPlayerCameraManager _returnvalue))
  (bind _returnvalue_3 (Transformation|GetWorldRotation _defaultsceneroot_2))
  (bind _transformcomponent (Variables|/Script/Engine.PlayerCameraManager|GetTransformComponent _playercameramanager))
  (bind _returnvalue_4 (- (.yaw _returnvalue_3) 1.8e+02))
  (bind _returnvalue_5 (Math|Rotator|MakeRotator (.roll _returnvalue_3) (.pitch _returnvalue_3) _returnvalue_4))
  (bind _returnvalue_6 (Math|Rotator|Delta(Rotator) _returnvalue_5 _returnvalue_2))
  (Transformation|SetWorldLocationAndRotation (Variables|/Game/Blueprints/Portal.Portal_C|GetPortalView (Variables|Default|GetDestination)) (+ (Math|Vector|RotateVector (Transformation|GetWorldLocation _transformcomponent) _returnvalue_6) (- (Transformation|GetWorldLocation _defaultsceneroot_2) (Math|Vector|RotateVector (Transformation|GetWorldLocation _defaultsceneroot) _returnvalue_6))) (Math|Rotator|CombineRotators (Transformation|GetWorldRotation _transformcomponent) _returnvalue_6) false false))

(fn ConstructionScript
  (Variables|/Script/Engine.SceneCaptureComponent2D|SetTextureTarget (Variables|Default|GetPortalView) (Variables|Default|GetTextureTarget)))