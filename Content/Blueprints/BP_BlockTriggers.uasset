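; BP_BlockTriggers is a trigger volume that springs a mid-game event blocking off the level.
; When the first-person character overlaps it, it checks that the game mode has more than one page picked up, candle moonlight initialized and blocks not yet spawned.
; It then calls MakeBlocksAppear on the game mode and force-closes the first BP_DoorWide tagged "base".
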(event OnComponentBeginOverlap(SpawnBlockTrigger)
  (params (OverlappedComponent :type Primitive%20Component%20Object%20Reference) (OtherActor :type Actor%20Object%20Reference) (OtherComp :type Primitive%20Component%20Object%20Reference) (OtherBodyIndex :type Integer) (bFromSweep :type Boolean) (SweepResult :type Hit%20Result%20Structure%20%28by%20ref%29))
  (bind _returnvalue (Game|GetGameMode))
  (bind _asthird_person_game_mode (Utilities|Casting|CastToThirdPersonGameMode _returnvalue))
  (Utilities|Casting|CastToFirstPersonCharacter OtherActor)
  (if (Math|Boolean|ANDBoolean (> (Variables|/Game/ThirdPersonBP/Blueprints/ThirdPersonGameMode.ThirdPersonGameMode_C|GetPagesPickedUp _asthird_person_game_mode) 1) (not (Variables|/Game/ThirdPersonBP/Blueprints/ThirdPersonGameMode.ThirdPersonGameMode_C|GetBlocksSpawned _asthird_person_game_mode)) (Variables|/Game/ThirdPersonBP/Blueprints/ThirdPersonGameMode.ThirdPersonGameMode_C|GetCandle/Moonlight%20Initialized _asthird_person_game_mode))
    (Default|MakeBlocksAppear (.AsThird%20Person%20Game%20Mode (Utilities|Casting|CastToThirdPersonGameMode (Game|GetGameMode))))
    (bind _outactors (Actor|GetAllActorsOfClass "/Game/HQ_ResidentialHouse/Actors/BP_DoorWide.BP_DoorWide_C"))
    (bind _array_element (Utilities|Array|ForEachLoopwithBreak _outactors :!label _label)
      (:LoopBody
        (if (Actor|ActorHasTag _array_element "base")
          (Default|ForceClosed _array_element)
          (goto _label Break))))))

(event EventBeginPlay)

(event Collision|EventActorBeginOverlap
  (params (OtherActor :type Actor%20Object%20Reference)))

(event EventTick
  (params (DeltaSeconds :type Float%20%28single-precision%29)))

(fn ConstructionScript)