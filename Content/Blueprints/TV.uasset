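; Interactable TV that toggles screen, light and audio, and drives a one-time scare once exactly two puzzles are completed.
; The main trigger switches it on; a second trigger teleports the FloatingCam monster and forces its path.
; A timeline then blends the dynamic screen material and crossfades in ghost audio, followed by scripted phone text.
; Delays later flicker a light, toggle the TV, and switch off lit lightswitches, resetting the effect alongside them.
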(event OnComponentBeginOverlap(MainTrigger)
  (params (OverlappedComponent :type Primitive%20Component%20Object%20Reference) (OtherActor :type Actor%20Object%20Reference) (OtherComp :type Primitive%20Component%20Object%20Reference) (OtherBodyIndex :type Integer) (bFromSweep :type Boolean) (SweepResult :type Hit%20Result%20Structure%20%28by%20ref%29))
  (if (== OtherActor (Game|GetPlayerCharacter 0))
    (if (== (Variables|/Game/ThirdPersonBP/Blueprints/ThirdPersonGameMode.ThirdPersonGameMode_C|GetPuzzlesCompleted (.AsThird%20Person%20Game%20Mode (Utilities|Casting|CastToThirdPersonGameMode (Game|GetGameMode)))) 2)
      (if (not (Variables|Default|GetIsOn?))
        (Utilities|FlowControl|DoOnce false
          (:Completed
            (CallFunction|Interact)))))))

(event OnComponentBeginOverlap(SecondaryTrigger)
  (params (OverlappedComponent :type Primitive%20Component%20Object%20Reference) (OtherActor :type Actor%20Object%20Reference) (OtherComp :type Primitive%20Component%20Object%20Reference) (OtherBodyIndex :type Integer) (bFromSweep :type Boolean) (SweepResult :type Hit%20Result%20Structure%20%28by%20ref%29))
  (bind _monster (Variables|Default|GetMonster))
  (bind _forcelocactor (Variables|Default|GetForceLocActor))
  (bind _returnvalue (Transformation|GetActorLocation _forcelocactor))
  (if (== OtherActor (Game|GetPlayerCharacter 0))
    (if (== (Variables|/Game/ThirdPersonBP/Blueprints/ThirdPersonGameMode.ThirdPersonGameMode_C|GetPuzzlesCompleted (.AsThird%20Person%20Game%20Mode (Utilities|Casting|CastToThirdPersonGameMode (Game|GetGameMode)))) 2)
      (Utilities|FlowControl|DoOnce false
        (:Completed
          (Class|NavMovementComponent|StopActiveMovement (Variables|/Script/Engine.Character|GetCharacterMovement _monster))
          (Transformation|SetActorLocationAndRotation _monster (Math|Vector|MakeVector (.x _returnvalue) (.y _returnvalue) (+ (.z _returnvalue) 81.0)) (Transformation|GetActorRotation _forcelocactor))
          (Default|ForcePath _monster (Variables|Default|GetForced%20Chosen%20Node))
          (bind _alpha (Timeline|FadeIn PlayFromStart)
            (:Update
              (Rendering|Material|SetScalarParameterValue (Variables|Default|GetOn) "Blend" (Math|Float|Lerp 0.0 1.0 _alpha) :!class /Script/Engine.MaterialInstanceDynamic)
              (Audio|Components|Audio|SetVolumeMultiplier (Variables|Default|GetghostsoundsTV) (Math|Float|Lerp 0.0 1.0 _alpha) :!class /Script/Engine.AudioComponent)
              (Audio|Components|Audio|SetVolumeMultiplier (Variables|Default|GetAudio) (Math|Float|Lerp 1.0 0.25 _alpha) :!class /Script/Engine.AudioComponent))
            (:Finished
              (bind _foundwidgets (Widget|GetAllWidgetsOfClass "/Game/Blueprints/Cellphone/WID_CellPhoneMaster.WID_CellPhoneMaster_C" false))
              (Default|ScriptedText (Utilities|Array|Get(acopy) _foundwidgets) "tv")
              (Utilities|FlowControl|Sequence
                (:then_0
                  (Utilities|FlowControl|Delay 15.0)
                  (Default|IFlickerShort (Variables|Default|GetLight) false))
                (:then_1
                  (Utilities|FlowControl|Delay (Variables|Default|GetRuntime))
                  (CallFunction|Interact)
                  (for _array_element (Utilities|Array|MakeArray (Variables|Default|GetLightswitch1) (Variables|Default|GetLightswitch2))
                    (if (Variables|/Game/LightSwitch.LightSwitch_C|GetIsOn? _array_element)
                      (Default|Interact _array_element)
                      (Audio|Components|Audio|SetVolumeMultiplier (Variables|Default|GetghostsoundsTV) 0.0 :!class /Script/Engine.AudioComponent)
                      (Audio|Components|Audio|SetVolumeMultiplier (Variables|Default|GetAudio) 1.0 :!class /Script/Engine.AudioComponent)
                      (Rendering|Material|SetScalarParameterValue (Variables|Default|GetOn) "Blend" 0.0 :!class /Script/Engine.MaterialInstanceDynamic))))))))))))

(event EventBeginPlay
  (bind _outactors (Actor|GetAllActorsOfClass "/Game/FirstPersonBP/Blueprints/FloatingCam.FloatingCam_C"))
  (for _array_element _outactors
    (Variables|Default|SetMonster _array_element)))

(event EventInteract
  (params (HitComponent :type Actor%20Component%20Object%20Reference))
  (bind _pointlight (Variables|Default|GetPointLight))
  (bind _audio (Variables|Default|GetAudio))
  (if (Variables|Default|GetIsOn?)
    (Rendering|Material|SetMaterial (Variables|Default|GetSM_TvScreen) 1 (Variables|Default|GetTurnedOff))
    (Rendering|SetVisibility _pointlight false false)
    (Audio|Components|Audio|Stop _audio)
    (Variables|Default|SetIsOn? false)
    (else
      (Rendering|Material|SetMaterial (Variables|Default|GetSM_TvScreen) 1 (Variables|Default|GetOn))
      (Rendering|SetVisibility _pointlight true false)
      (Audio|Components|Audio|Play _audio 0.0)
      (Variables|Default|SetIsOn? true))))

(fn ConstructionScript
  (bind _returnvalue (Rendering|Material|CreateDynamicMaterialInstance "/Game/SciFiGlitchPostPro/PostProcess/Instance/Static_Inst.Static_Inst" "None" :!class /Script/Engine.KismetMaterialLibrary))
  (Variables|Default|SetOn _returnvalue))