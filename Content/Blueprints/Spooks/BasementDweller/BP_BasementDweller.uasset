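; Basement dweller scare that reveals a hidden Dweller when the player enters its trigger, once the game mode's candle/moonlight flag is initialized.
; The reveal fires once, forcing the referenced lamp on and swinging it.
; After 40 seconds or a qualifying trigger exit, a shared one-shot plays the lamp animation, flickers it and dissolves the Dweller.
; An Entering flag, cleared by the LEAVINGROOM volume, gates both trigger responses by direction.
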(event OnComponentBeginOverlap(DwellerTrigger)
  (params (OverlappedComponent :type Primitive%20Component%20Object%20Reference) (OtherActor :type Actor%20Object%20Reference) (OtherComp :type Primitive%20Component%20Object%20Reference) (OtherBodyIndex :type Integer) (bFromSweep :type Boolean) (SweepResult :type Hit%20Result%20Structure%20%28by%20ref%29))
  (bind _asthird_person_game_mode (Utilities|Casting|CastToThirdPersonGameMode (Game|GetGameMode)))
  (if (Math|Boolean|ANDBoolean (Actor|ActorHasTag OtherActor "player") (Variables|/Game/ThirdPersonBP/Blueprints/ThirdPersonGameMode.ThirdPersonGameMode_C|GetCandle/Moonlight%20Initialized _asthird_person_game_mode) (Variables|Default|Getentering))
    (Utilities|FlowControl|DoOnce false
      (:Completed
        (Class|LightInterface|IForceon(Message) (Variables|Default|GetLamp))
        (Rendering|SetVisibility (Variables|/Script/Engine.Actor|GetRootComponent (Variables|Default|GetDweller)) true false)
        (bind _asbp_lamp_swinging (Utilities|Casting|CastToBP_LampSwinging (Variables|Default|GetLamp)))
        (Default|SwingLight _asbp_lamp_swinging)
        (Utilities|FlowControl|Delay 4e+01)
        (Utilities|FlowControl|DoOnce false
          (:Completed
            (bind _asbp_lamp_swinging_2 (Utilities|Casting|CastToBP_LampSwinging (Variables|Default|GetLamp)))
            (Components|Animation|PlayAnimation (Variables|/Game/HQ_ResidentialHouse/Actors/BP_LampSwinging.BP_LampSwinging_C|GetSkeletalMesh _asbp_lamp_swinging_2) 0 false)
            (Class|LightInterface|IFlickerShort(Message) (Variables|Default|GetLamp) true)
            (Default|DissolveDweller (Variables|Default|GetDweller))))))))

(event OnComponentEndOverlap(DwellerTrigger)
  (params (OverlappedComponent :type Primitive%20Component%20Object%20Reference) (OtherActor :type Actor%20Object%20Reference) (OtherComp :type Primitive%20Component%20Object%20Reference) (OtherBodyIndex :type Integer))
  (if (Math|Boolean|ANDBoolean (Actor|ActorHasTag OtherActor "player") (Variables|/Game/ThirdPersonBP/Blueprints/ThirdPersonGameMode.ThirdPersonGameMode_C|GetCandle/Moonlight%20Initialized (Variables|Default|GetGameMode)) (Variables|Default|Getentering))
    (Utilities|FlowControl|DoOnce false
      (:Completed
        (bind _asbp_lamp_swinging (Utilities|Casting|CastToBP_LampSwinging (Variables|Default|GetLamp)))
        (Components|Animation|PlayAnimation (Variables|/Game/HQ_ResidentialHouse/Actors/BP_LampSwinging.BP_LampSwinging_C|GetSkeletalMesh _asbp_lamp_swinging) 0 false)
        (Class|LightInterface|IFlickerShort(Message) (Variables|Default|GetLamp) true)
        (Default|DissolveDweller (Variables|Default|GetDweller))))
    (else
      (Variables|Default|Setentering true))))

(event OnComponentBeginOverlap(LEAVINGROOM)
  (params (OverlappedComponent :type Primitive%20Component%20Object%20Reference) (OtherActor :type Actor%20Object%20Reference) (OtherComp :type Primitive%20Component%20Object%20Reference) (OtherBodyIndex :type Integer) (bFromSweep :type Boolean) (SweepResult :type Hit%20Result%20Structure%20%28by%20ref%29))
  (if (Actor|ActorHasTag OtherActor "player")
    (Variables|Default|Setentering false)))

(event EventBeginPlay
  (bind _asthird_person_game_mode (Utilities|Casting|CastToThirdPersonGameMode (Game|GetGameMode)))
  (Variables|Default|SetGameMode _asthird_person_game_mode)
  (Rendering|SetVisibility (Variables|/Script/Engine.Actor|GetRootComponent (Variables|Default|GetDweller)) false false))

(event Collision|EventActorBeginOverlap
  (params (OtherActor :type Actor%20Object%20Reference)))

(event EventTick
  (params (DeltaSeconds :type Float%20%28single-precision%29)))

(fn ConstructionScript)