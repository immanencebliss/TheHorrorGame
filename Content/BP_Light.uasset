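; Switchable light actor that can be forced on or off or flickered via interface events.
; Construction script caches point lights and their default intensity, creates dynamic mesh materials and applies IsOff.
; Events set point light intensity and "Emission Intensity" together, with three timelines driving long, short and looping flickers.
; Only the last material instance is stored, spot and rect lights are gathered but unused, and ToggleLight ignores Off.
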(event EventBeginPlay)

(event EventIForceOff
  ;[1 1 1] Toggle Light
  (for _array_element (Variables|Default|GetPoints)
    (Rendering|Components|Light|SetIntensity _array_element 0.0)
    (Rendering|Material|SetScalarParameterValue (Variables|Default|GetMatInstance) "Emission Intensity" 0.0 :!class /Script/Engine.MaterialInstanceDynamic)
    (Variables|Default|SetIsOff? true)))

(event EventIForceon
  ;[1 1 1] Toggle Light
  (for _array_element (Variables|Default|GetPoints)
    (Rendering|Components|Light|SetIntensity _array_element (Variables|Default|GetDefault%20Intensity))
    (Rendering|Material|SetScalarParameterValue (Variables|Default|GetMatInstance) "Emission Intensity" 15.0 :!class /Script/Engine.MaterialInstanceDynamic)
    (Variables|Default|SetIsOff? false)))

(event EventIFlickerLong
  (params (FlickOn :type Boolean))
  ;[1 1 1] Flicker lights long
  (bind _output_get (Variables|Default|SetFlickOn FlickOn))
  (if _output_get
    (bind _brightness (Timeline|Timeline_1 PlayFromStart)
      (:Update
        (for _array_element (Variables|Default|GetPoints)
          (Rendering|Components|Light|SetIntensity _array_element (Math|Float|Lerp 0.0 (Variables|Default|GetDefault%20Intensity) (/ _brightness 1e+01)))
          (if (Variables|Default|GetFlickOn)
            (Rendering|Material|SetScalarParameterValue (Variables|Default|GetMatInstance) "Emission Intensity" (Math|Float|Lerp 0.0 15.0 (/ _brightness 1e+01)) :!class /Script/Engine.MaterialInstanceDynamic)
            (Variables|Default|SetIsOff? false)
            (else
              (Rendering|Material|SetScalarParameterValue (Variables|Default|GetMatInstance) "Emission Intensity" (Math|Float|Lerp 0.0 15.0 (/ _brightness 1e+01)) :!class /Script/Engine.MaterialInstanceDynamic)
              (Variables|Default|SetIsOff? true))))))
    (else
      (Timeline|Timeline_1 ReverseFromEnd))))

(event EventIFlickerShort
  (params (FlickOn :type Boolean))
  ;[1 1 1] Flicker lights Short
  (bind _output_get (Variables|Default|SetFlickOn FlickOn))
  (if _output_get
    (bind _flicker_style_1 (Timeline|Timeline_2 ReverseFromEnd)
      (:Update
        (for _array_element (Variables|Default|GetPoints)
          (Rendering|Components|Light|SetIntensity _array_element (Math|Float|Lerp 0.0 (Variables|Default|GetDefault%20Intensity) _flicker_style_1))
          (if (Variables|Default|GetFlickOn)
            (Rendering|Material|SetScalarParameterValue (Variables|Default|GetMatInstance) "Emission Intensity" (Math|Float|Lerp 0.0 15.0 _flicker_style_1) :!class /Script/Engine.MaterialInstanceDynamic)
            (Variables|Default|SetIsOff? false)
            (else
              (Rendering|Material|SetScalarParameterValue (Variables|Default|GetMatInstance) "Emission Intensity" (Math|Float|Lerp 0.0 15.0 _flicker_style_1) :!class /Script/Engine.MaterialInstanceDynamic)
              (Variables|Default|SetIsOff? true))))))
    (else
      (Timeline|Timeline_2 PlayFromStart))))

(event EventToggleLight
  (params (Off? :type Boolean))
  ;[1 1 1] Toggle Light
  (for _array_element (Variables|Default|GetPoints)
    (Rendering|Components|Light|SetIntensity _array_element (Variables|Default|GetDefault%20Intensity))
    (Rendering|Material|SetScalarParameterValue (Variables|Default|GetMatInstance) "Emission Intensity" 15.0 :!class /Script/Engine.MaterialInstanceDynamic)
    (Variables|Default|SetIsOff? false)))

(event EventIFlickeron
  (params (FlickOn :type Boolean))
  ;[1 1 1] Flicker lights Looping
  (bind _output_get (Variables|Default|SetFlickOn FlickOn))
  (if _output_get
    (bind _newtrack_0 (Timeline|Timeline_0 ReverseFromEnd)
      (:Update
        (for _array_element (Variables|Default|GetPoints)
          (Rendering|Components|Light|SetIntensity _array_element (Math|Float|Lerp 0.0 (Variables|Default|GetDefault%20Intensity) _newtrack_0))
          (if (Variables|Default|GetFlickOn)
            (Rendering|Material|SetScalarParameterValue (Variables|Default|GetMatInstance) "Emission Intensity" (Math|Float|Lerp 0.0 15.0 _newtrack_0) :!class /Script/Engine.MaterialInstanceDynamic)
            (Variables|Default|SetIsOff? false)
            (else
              (Rendering|Material|SetScalarParameterValue (Variables|Default|GetMatInstance) "Emission Intensity" (Math|Float|Lerp 0.0 15.0 _newtrack_0) :!class /Script/Engine.MaterialInstanceDynamic)
              (Variables|Default|SetIsOff? true))))))
    (else
      (Timeline|Timeline_0 PlayFromStart))))

(event EventIFlickerOff
  (params (FlickOn :type Boolean))
  ;[1 1 1] Flicker lights Looping
  (Utilities|FlowControl|Sequence
    (:then_0
      (bind _newtrack_0 (Timeline|Timeline_0 Stop)
        (:Update
          (for _array_element (Variables|Default|GetPoints)
            (Rendering|Components|Light|SetIntensity _array_element (Math|Float|Lerp 0.0 (Variables|Default|GetDefault%20Intensity) _newtrack_0))
            (if (Variables|Default|GetFlickOn)
              (Rendering|Material|SetScalarParameterValue (Variables|Default|GetMatInstance) "Emission Intensity" (Math|Float|Lerp 0.0 15.0 _newtrack_0) :!class /Script/Engine.MaterialInstanceDynamic)
              (Variables|Default|SetIsOff? false)
              (else
                (Rendering|Material|SetScalarParameterValue (Variables|Default|GetMatInstance) "Emission Intensity" (Math|Float|Lerp 0.0 15.0 _newtrack_0) :!class /Script/Engine.MaterialInstanceDynamic)
                (Variables|Default|SetIsOff? true)))))))
    (:then_1
      (if FlickOn
        (for _array_element_2 (Variables|Default|GetPoints)
          (Rendering|Components|Light|SetIntensity _array_element_2 (Variables|Default|GetDefault%20Intensity))
          (if (Variables|Default|GetFlickOn)
            (Rendering|Material|SetScalarParameterValue (Variables|Default|GetMatInstance) "Emission Intensity" (Math|Float|Lerp 0.0 15.0 _newtrack_0) :!class /Script/Engine.MaterialInstanceDynamic)
            (Variables|Default|SetIsOff? false)
            (else
              (Rendering|Material|SetScalarParameterValue (Variables|Default|GetMatInstance) "Emission Intensity" (Math|Float|Lerp 0.0 15.0 _newtrack_0) :!class /Script/Engine.MaterialInstanceDynamic)
              (Variables|Default|SetIsOff? true))))
        (else
          (for _array_element_3 (Variables|Default|GetPoints)
            (Rendering|Components|Light|SetIntensity _array_element_3 0.0)
            (if (Variables|Default|GetFlickOn)
              (Rendering|Material|SetScalarParameterValue (Variables|Default|GetMatInstance) "Emission Intensity" (Math|Float|Lerp 0.0 15.0 _newtrack_0) :!class /Script/Engine.MaterialInstanceDynamic)
              (Variables|Default|SetIsOff? false)
              (else
                (Rendering|Material|SetScalarParameterValue (Variables|Default|GetMatInstance) "Emission Intensity" (Math|Float|Lerp 0.0 15.0 _newtrack_0) :!class /Script/Engine.MaterialInstanceDynamic)
                (Variables|Default|SetIsOff? true)))))))))

(event EventToggleLightOff
  (params (Off? :type Boolean))
  ;[1 1 1] Toggle Light
  (for _array_element (Variables|Default|GetPoints)
    (Rendering|Components|Light|SetIntensity _array_element 0.0)
    (Rendering|Material|SetScalarParameterValue (Variables|Default|GetMatInstance) "Emission Intensity" 0.0 :!class /Script/Engine.MaterialInstanceDynamic)
    (Variables|Default|SetIsOff? true)))

(fn ConstructionScript
  (Utilities|FlowControl|Sequence
    (:then_0
      (bind _output_get (Variables|Default|SetPoints (Actor|GetComponentsByClass "/Script/Engine.PointLightComponent")))
      (Variables|Default|SetDefault%20Intensity (Variables|/Script/Engine.LightComponentBase|GetIntensity (Utilities|Array|Get(acopy) _output_get))))
    (:then_1
      (Variables|Default|SetSpots (Actor|GetComponentsByClass "/Script/Engine.SpotLightComponent")))
    (:then_2
      (Variables|Default|SetRects (Actor|GetComponentsByClass "/Script/Engine.RectLightComponent")))
    (:then_3
      (bind _output_get_2 (Variables|Default|Setmeshes (Actor|GetComponentsByClass "/Script/Engine.StaticMeshComponent")))
      (for _array_element _output_get_2
        (bind _returnvalue (Rendering|Material|CreateDynamicMaterialInstance _array_element 0 (Rendering|Material|GetMaterial _array_element 0) "None" :!class /Script/Engine.PrimitiveComponent))
        (Variables|Default|SetMatInstance _returnvalue)
        (for _array_element_2 (Variables|Default|GetPoints)
          (if (Variables|Default|GetIsOff?)
            (Rendering|Components|Light|SetIntensity _array_element_2 0.0)
            (Rendering|Material|SetScalarParameterValue (Variables|Default|GetMatInstance) "Emission Intensity" 0.0 :!class /Script/Engine.MaterialInstanceDynamic)
            (else
              (Rendering|Components|Light|SetIntensity _array_element_2 (Variables|Default|GetDefault%20Intensity))
              (Rendering|Material|SetScalarParameterValue (Variables|Default|GetMatInstance) "Emission Intensity" 15.0 :!class /Script/Engine.MaterialInstanceDynamic))))))))